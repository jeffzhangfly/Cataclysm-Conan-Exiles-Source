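; Mod controller for the Cataclysm mod that injects its custom content into the game's data tables.
; ModDataTableOperations merges the mod's tables into the base spawn, weighted spawn, equipment, profession, stat, item, recipe, NPC dialogue, monster stat, map marker and race tables.
; The stat template table receives separate boss and monster tables.
; The event graph and construction script are empty, so all logic lives in those merges.
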(event EventBeginPlay)

(event EventTick
  (params (DeltaSeconds :type Float%20%28single-precision%29)))

(fn ConstructionScript)

(fn ModDataTableOperations
  (Class|ModController|MergeDataTables "/Game/Systems/SpawnTable/SpawnDataTable.SpawnDataTable" "/Game/Mods/Cat_Mod2f/Data_tables/NPC/Cataclysmspawndata_Mobs.Cataclysmspawndata_Mobs")
  (Class|ModController|MergeDataTables "/Game/Systems/SpawnTable/WeightedSpawnTableRow.WeightedSpawnTableRow" "/Game/Mods/Cat_Mod2f/Data_tables/NPC/Cataclysm_weightedspawn.Cataclysm_weightedspawn")
  (Class|ModController|MergeDataTables "/Game/Systems/SpawnTable/EquipmentTemplateDataTable.EquipmentTemplateDataTable" "/Game/Mods/Cat_Mod2f/Data_tables/NPC/Cataclysm_Equipment_template.Cataclysm_Equipment_template")
  (Class|ModController|MergeDataTables "/Game/Systems/SpawnTable/ProfessionTemplateDataTable.ProfessionTemplateDataTable" "/Game/Mods/Cat_Mod2f/Data_tables/NPC/Cataclysm_profession_template.Cataclysm_profession_template")
  (Class|ModController|MergeDataTables "/Game/Systems/SpawnTable/StatTemplateDataTable.StatTemplateDataTable" "/Game/Mods/Cat_Mod2f/Data_tables/NPC/Cataclysm_Stattemplatedatatable_boss.Cataclysm_Stattemplatedatatable_boss")
  (Class|ModController|MergeDataTables "/Game/Systems/SpawnTable/StatTemplateDataTable.StatTemplateDataTable" "/Game/Mods/Cat_Mod2f/Data_tables/NPC/Cataclysm_Stattemplatedatatable_monsters.Cataclysm_Stattemplatedatatable_monsters")
  (Class|ModController|MergeDataTables "/Game/Items/ItemTable.ItemTable" "/Game/Mods/Cat_Mod2f/Data_tables/Items/CataclysmServermod2_itemTable.CataclysmServermod2_itemTable")
  (Class|ModController|MergeDataTables "/Game/Items/Recipes/RecipesTable.RecipesTable" "/Game/Mods/Cat_Mod2f/Data_tables/Items/Cataclysm_Recipe_table.Cataclysm_Recipe_table")
  (Class|ModController|MergeDataTables "/Game/Systems/Dialogue/NpcDialogues.NpcDialogues" "/Game/Mods/Cat_Mod2f/Data_tables/NPC/Cataclysm_Dialogue.Cataclysm_Dialogue")
  (Class|ModController|MergeDataTables "/Game/Characters/NPCs/MonsterStatTable.MonsterStatTable" "/Game/Mods/Cat_Mod2f/Data_tables/NPC/Cataclysm_MonsterStatTable.Cataclysm_MonsterStatTable")
  (Class|ModController|MergeDataTables "/Game/Systems/Map/MapMarkers.MapMarkers" "/Game/Mods/Cat_Mod2f/Data_tables/MapMarkers/Cataclysm_Map_Markers.Cataclysm_Map_Markers")
  (Class|ModController|MergeDataTables "/Game/Systems/SpawnTable/RaceTemplateDataTable.RaceTemplateDataTable" "/Game/Mods/Cat_Mod2f/Data_tables/NPC/Cataclysm_raceTemplate.Cataclysm_raceTemplate"))